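; Level-exit door actor that stays hidden until the player's soul count for its level reaches the required amount.
; Tick toggles visibility from the ALS character's per-level soul map and plays a low-pitched sound once upon unlocking.
; Overlapping the plane while visible flies the character through the start-level list in sequence, setting the current level and easing to each entry's position and arrow rotation, then ends flight.
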(event `self.ReceiveBeginPlay`
  (bind _asals_anim_man_character_bp (cast `/Game/AdvancedLocomotionV4/Blueprints/CharacterLogic/ALS_AnimMan_CharacterBP` (`GameplayStatics.GetPlayerPawn` 0)))
  (set `self.Character` _asals_anim_man_character_bp))

(event `self.ReceiveTick`
  (params (DeltaSeconds :type "Float (single-precision)"))
  (bind _character (`self.Character`))
  (bind _returnvalue (>= (`BlueprintMapLibrary.Map_Find` (`/Game/AdvancedLocomotionV4/Blueprints/CharacterLogic/ALS_AnimMan_CharacterBP.SoulsByLevel` _character) (`self.LevelName`)) (`self.SoulsNeeded`)))
  (`/Engine/EditorBlueprintResources/StandardMacros.IsValid` _character
    (:`Is Valid`
      (`self.SetActorHiddenInGame` (not _returnvalue))
      (if _returnvalue
        (`/Engine/EditorBlueprintResources/StandardMacros.DoOnce` false :!label _label
          (:`Completed`
            (`GameplayStatics.PlaySoundAtLocation` "/Engine/EditorSounds/GamePreview/EndPlayInEditor_Cue.EndPlayInEditor_Cue" (`SceneComponent.K2_GetComponentLocation` (`self.StaticMesh`)) (struct) 0.2 0.2 0.0 null null null)))
        (else
          (goto _label :!via `Reset`))))))

(event `self.Plane.OnComponentBeginOverlap`
  (params (OverlappedComponent :type "PrimitiveComponent Object Reference") (OtherActor :type "Actor Object Reference") (OtherComp :type "PrimitiveComponent Object Reference") (OtherBodyIndex :type Integer) (bFromSweep :type Boolean) (SweepResult :type "HitResult Structure (by ref)"))
  (bind _startlevellist (`self.StartLevelList`))
  (bind _currentstartlevel (`self.CurrentStartLevel`))
  (bind _output (`|GetArrayItem` _startlevellist _currentstartlevel))
  (bind _asals_anim_man_character_bp (cast `/Game/AdvancedLocomotionV4/Blueprints/CharacterLogic/ALS_AnimMan_CharacterBP` OtherActor))
  (if (not (`self.bHidden`))
    (if (> (`KismetArrayLibrary.Array_Length` _startlevellist) _currentstartlevel) :!label _label_2
      (`/Engine/EditorBlueprintResources/StandardMacros.IsValid` _output
        (:`Is Valid`
          (bind _output_get (set `self.CurrentStartLevelObj` _output))
          (bind _result (`/Engine/EditorBlueprintResources/StandardMacros.IncrementInt` (`self.CurrentStartLevel`))
            (:`  `
              (`/Game/AdvancedLocomotionV4/Blueprints/CharacterLogic/ALS_AnimMan_CharacterBP.SetCurrentLevel` _asals_anim_man_character_bp (`/Game/Blueprints/BP_StartLevel.Level` _output_get))
              (set `self.CurrentStartLevel` _result)
              (`/Game/AdvancedLocomotionV4/Blueprints/CharacterLogic/ALS_AnimMan_CharacterBP.Fly` _asals_anim_man_character_bp true)
              (`KismetSystemLibrary.MoveComponentTo` (`Actor.RootComponent` _asals_anim_man_character_bp) (`SceneComponent.K2_GetComponentLocation` (`Actor.RootComponent` _output_get)) (`SceneComponent.K2_GetComponentRotation` (`/Game/Blueprints/BP_StartLevel.Arrow` _output_get)) true true 1.0)
              (goto _label_2))))
        (:`Is Not Valid`
          _)))
    (set `self.CurrentStartLevel` 0)
    (`/Game/AdvancedLocomotionV4/Blueprints/CharacterLogic/ALS_AnimMan_CharacterBP.Fly` _asals_anim_man_character_bp false)))

(fn `UserConstructionScript`)