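; BP_PreviousLevel is a trigger that sends the ALS player character back through a chain of level start points.
; Box overlap sets the character's current level to ResetLevel, then, unless Hidden, walks StartLevelList in order.
; Each entry updates the character's level and glides it to that start's location and arrow rotation via looped, eased MoveComponentTo calls.
; Fly mode stays on during travel, switching off and resetting the index at the list's end or an invalid entry.
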(event `self.Box.OnComponentBeginOverlap`
  (params (OverlappedComponent :type "PrimitiveComponent Object Reference") (OtherActor :type "Actor Object Reference") (OtherComp :type "PrimitiveComponent Object Reference") (OtherBodyIndex :type Integer) (bFromSweep :type Boolean) (SweepResult :type "HitResult Structure (by ref)"))
  (bind _startlevellist (`self.StartLevelList`))
  (bind _currentstartlevel (`self.CurrentStartLevel`))
  (bind _output (`|GetArrayItem` _startlevellist _currentstartlevel))
  (bind _asals_anim_man_character_bp (cast `/Game/AdvancedLocomotionV4/Blueprints/CharacterLogic/ALS_AnimMan_CharacterBP` OtherActor))
  (`/Game/AdvancedLocomotionV4/Blueprints/CharacterLogic/ALS_AnimMan_CharacterBP.SetCurrentLevel` _asals_anim_man_character_bp (`self.ResetLevel`))
  (if (not (`self.bHidden`))
    (if (> (`KismetArrayLibrary.Array_Length` _startlevellist) _currentstartlevel) :!label _label
      (`/Engine/EditorBlueprintResources/StandardMacros.IsValid` _output
        (:`Is Valid`
          (bind _output_get (set `self.CurrentStartLevelObj` _output))
          (bind _result (`/Engine/EditorBlueprintResources/StandardMacros.IncrementInt` (`self.CurrentStartLevel`))
            (:`  `
              (`/Game/AdvancedLocomotionV4/Blueprints/CharacterLogic/ALS_AnimMan_CharacterBP.SetCurrentLevel` _asals_anim_man_character_bp (`/Game/Blueprints/BP_StartLevel.Level` _output_get))
              (set `self.CurrentStartLevel` _result)
              (`/Game/AdvancedLocomotionV4/Blueprints/CharacterLogic/ALS_AnimMan_CharacterBP.Fly` _asals_anim_man_character_bp true)
              (`KismetSystemLibrary.MoveComponentTo` (`Actor.RootComponent` _asals_anim_man_character_bp) (`SceneComponent.K2_GetComponentLocation` (`Actor.RootComponent` _output_get)) (`SceneComponent.K2_GetComponentRotation` (`/Game/Blueprints/BP_StartLevel.Arrow` _output_get)) true true 1.0)
              (goto _label))))
        (:`Is Not Valid`
          _)))
    (set `self.CurrentStartLevel` 0)
    (`/Game/AdvancedLocomotionV4/Blueprints/CharacterLogic/ALS_AnimMan_CharacterBP.Fly` _asals_anim_man_character_bp false)))

(fn `UserConstructionScript`)