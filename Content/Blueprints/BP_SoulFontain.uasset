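; Soul fountain actor whose Niagara effect hops between five path components and launches the player character skyward on overlap.
; Each time the effect finishes, it unbinds the current path, waits a random sub-second delay, moves to the next path and restarts.
; Only the active path's overlap is bound, launching any ALS_AnimMan character strongly upward with slight random horizontal drift.
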(event `self.ReceiveBeginPlay`
  (set `self.PathList` (`|MakeArray` (`self.Path1`) (`self.Path2`) (`self.Path3`) (`self.Path4`) (`self.Path5`))))

(event `self.Niagara.OnSystemFinished`
  (params (PSystem :type "NiagaraComponent Object Reference"))
  (bind _currentpath (`self.CurrentPath`))
  (`/Engine/EditorBlueprintResources/StandardMacros.IsValid` _currentpath
    (:`Is Valid`
      (clear `PrimitiveComponent.OnComponentBeginOverlap` _currentpath))
    (:`Is Not Valid`
      _))
  (`KismetSystemLibrary.Delay` (`KismetMathLibrary.RandomFloat`))
  (bind _newarrayitem (`/Game/AdvancedLocomotionV4/Blueprints/Libraries/ALS_MacroLibrary.ML_GetNextArrayItem` (`self.PathList`) (`self.CurrentPath`)))
  (`SceneComponent.K2_SetWorldLocation` (`self.Niagara`) (`SceneComponent.K2_GetComponentLocation` _newarrayitem) false true)
  (set `self.CurrentPath` _newarrayitem)
  (`NiagaraComponent.ReinitializeSystem` (`self.Niagara`))
  (add `PrimitiveComponent.OnComponentBeginOverlap` (`self.CurrentPath`) (delegate `PlayerCollision`)))

(event `PlayerCollision`
  (params (OverlappedComponent :type "PrimitiveComponent Object Reference") (OtherActor :type "Actor Object Reference") (OtherComp :type "PrimitiveComponent Object Reference") (OtherBodyIndex :type Integer) (bFromSweep :type Boolean) (SweepResult :type "HitResult Structure (by ref)"))
  (bind _asals_anim_man_character_bp (cast `/Game/AdvancedLocomotionV4/Blueprints/CharacterLogic/ALS_AnimMan_CharacterBP` OtherActor))
  (`Character.LaunchCharacter` _asals_anim_man_character_bp (`KismetMathLibrary.MakeVector` (* (`KismetMathLibrary.RandomFloat`) 100.0) (* (`KismetMathLibrary.RandomFloat`) 100.0) 2000.0) false false))

(fn `UserConstructionScript`)